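; BP_CrystalBig is a large crystal actor that breaks into a small crystal when damaged enough.
; AnyDamage subtracts damage from an integer Health value; at zero or below, it spawns BP_Crystal_Small at its location and rotation, then destroys itself.
; Disconnected nodes that would hide the Cube and disable the Box collision never run.
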(event `self.ReceiveAnyDamage`
  (params (Damage :type "Float (single-precision)") (DamageType :type "DamageType Object Reference") (InstigatedBy :type "Controller Object Reference") (DamageCauser :type "Actor Object Reference"))
  (bind _output_get (set `self.Health` (`KismetMathLibrary.FTrunc` (- (`self.Health`) Damage))))
  (if (<= _output_get 0)
    (`|SpawnActorFromClass` "/Game/Blueprints/Character/Inventory/BP_Crystal_Small.BP_Crystal_Small_C" (`KismetMathLibrary.MakeTransform` (`self.K2_GetActorLocation`) (`self.K2_GetActorRotation`)) "Undefined" "MultiplyWithRoot" null null)
    (`self.K2_DestroyActor`)))

(fn `UserConstructionScript`)