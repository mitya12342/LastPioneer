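; Character component for wall building: the player previews a WallDraft and places it by spending Crystals.
; IA_Build toggles build mode, where Tick runs a short camera line trace and moves a collision-free preview mesh, created once per session via DoOnce.
; The preview aligns to the surface normal with yaw from the view direction.
; IA_PlaceBuilding spawns the wall if the trace hits something other than a WallDraft and Crystals cover the cost.
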(event `self.ReceiveBeginPlay`
  (bind _aslpcharacter (cast `/Game/Blueprints/Character/LPCharacter` (`self.GetOwner`)))
  (set `self.Camera` (`/Game/Blueprints/Character/LPCharacter.Camera` _aslpcharacter))
  (set `self.CharBP` _aslpcharacter))

(event `ResetBuildMode`
  (goto _label :!via `Reset`))

(event `self.ReceiveTick`
  (params (DeltaSeconds :type "Float (single-precision)"))
  (if (`self.BuildMode`)
    (`self.PreviewLoop`)))

(event `PreviewLoop`
  (bind _preview_mesh (`self.Preview Mesh`))
  (bind (_returnvalue_location _returnvalue_rotation) (`KismetMathLibrary.BreakTransform` (`SceneComponent.K2_GetComponentToWorld` (`self.Camera`))))
  (bind (_outhit _returnvalue) (`KismetSystemLibrary.LineTraceSingle` _returnvalue_location (+ _returnvalue_location (* (`KismetMathLibrary.GetForwardVector` _returnvalue_rotation) 700.0)) "TraceTypeQuery1"))
  (set `self.ValidPlace` _returnvalue)
  (if _returnvalue
    (`|ExecutionSequence`
      (:`then_0`
        (`/Engine/EditorBlueprintResources/StandardMacros.DoOnce` false :!label _label
          (:`Completed`
            (bind _returnvalue_2 (`|AddComponentByClass` (`self.CharBP`) "/Script/Engine.StaticMeshComponent" false (`self.Build Preview Transform`)))
            (bind _output_get (set `self.Preview Mesh` _returnvalue_2))
            (`StaticMeshComponent.SetStaticMesh` _output_get "/Game/Props/Wall/WallDraftMesh.WallDraftMesh")
            (`PrimitiveComponent.SetMaterial` _output_get 0 "/Game/Blueprints/Character/BuildingPreview.BuildingPreview")
            (`PrimitiveComponent.SetCollisionEnabled` _output_get "NoCollision"))))
      (:`then_1`
        (bind (_bblockinghit _binitialoverlap _time _distance _location _impactpoint _normal _impactnormal _physmat _hitactor) (`GameplayStatics.BreakHitResult` _outhit))
        (cast `/Game/Props/Wall/WallDraft` _hitactor
          (:`then`
            (set `self.ValidPlace` false))
          (:`CastFailed`
            (bind (_returnvalue_roll _returnvalue_pitch) (`KismetMathLibrary.BreakRotator` (`KismetMathLibrary.Conv_VectorToRotator` _normal)))
            (bind (_returnvalue_roll_2 _returnvalue_pitch_2 _returnvalue_yaw) (`KismetMathLibrary.BreakRotator` (`KismetMathLibrary.Conv_VectorToRotator` (- _location _returnvalue_location))))
            (bind _output_get_2 (set `self.Build Preview Transform` (`KismetMathLibrary.MakeTransform` _location (`KismetMathLibrary.MakeRotator` _returnvalue_roll (+ _returnvalue_pitch -90.0) _returnvalue_yaw))))
            (`SceneComponent.K2_SetWorldTransform` _preview_mesh _output_get_2 false false)
            (`SceneComponent.SetVisibility` _preview_mesh (`self.ValidPlace`) true)))))))

(event `EnhancedInput|/Game/Blueprints/Character/Input/IA_Build`
  (params (ActionValue :type Boolean) (ElapsedSeconds :type "Float (double-precision)") (TriggeredSeconds :type "Float (double-precision)") (InputAction :type "InputAction Object Reference" :default "/Game/Blueprints/Character/Input/IA_Build.IA_Build"))
  (:`Started`
    (`/Engine/EditorBlueprintResources/StandardMacros.FlipFlop`
      (:`A`
        (set `self.BuildMode` true))
      (:`B`
        (set `self.BuildMode` false)
        (`StaticMeshComponent.SetStaticMesh` (`self.Preview Mesh`) null)
        (set `self.Preview Mesh` null)
        (`self.ResetBuildMode`)))))

(event `EnhancedInput|/Game/Blueprints/Character/Input/IA_PlaceBuilding`
  (params (ActionValue :type Boolean) (ElapsedSeconds :type "Float (double-precision)") (TriggeredSeconds :type "Float (double-precision)") (InputAction :type "InputAction Object Reference" :default "/Game/Blueprints/Character/Input/IA_PlaceBuilding.IA_PlaceBuilding"))
  (:`Started`
    (set `self.BuildingBudget` (`/Game/Blueprints/Character/LPCharacter.Crystals` (`self.CharBP`)))
    (if (and (`self.BuildMode`) (`self.ValidPlace`) (>= (`self.BuildingBudget`) (`self.BuildingCost`)))
      (`|SpawnActorFromClass` "/Game/Props/Wall/WallDraft.WallDraft_C" (`self.Build Preview Transform`) "AlwaysSpawn" "MultiplyWithRoot" null null)
      (set `/Game/Blueprints/Character/LPCharacter.Crystals` (- (`self.BuildingBudget`) (`self.BuildingCost`)) (`self.CharBP`)))))